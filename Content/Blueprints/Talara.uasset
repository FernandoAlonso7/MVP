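; Talara is a player-controlled Character Blueprint that handles movement, camera look, jumping and crouching through input mappings with Spanish names.
; Movimiento axes move it along the control rotation's forward and right vectors, while Vista axes feed controller yaw and pitch.
; Saltar jumps while held and stops on release, and Agacharse toggles crouch based on the movement component's current crouch state.
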(event Input|ActionEvents|InputActionSaltar
  (params (Key :type Key%20Structure))
  (:Pressed
    (Character|Jump))
  (:Released
    (Character|StopJumping)))

(event Input|ActionEvents|InputActionAgacharse
  (params (Key :type Key%20Structure))
  (:Pressed
    (if (AI|Components|NavMovement|IsCrouching (Variables|Character|GetCharacterMovement))
      (Character|UnCrouch)
      (else
        (Character|Crouch)))))

(event Input|AxisEvents|InputAxisMovimientoY
  (params (AxisValue :type Float%20%28single-precision%29))
  (Pawn|Input|AddMovementInput (Math|Vector|GetRightVector (Pawn|GetControlRotation :!class /Script/Engine.Pawn)) AxisValue false))

(event Input|AxisEvents|InputAxisMovimientoX
  (params (AxisValue :type Float%20%28single-precision%29))
  (Pawn|Input|AddMovementInput (Math|Vector|GetForwardVector (Pawn|GetControlRotation :!class /Script/Engine.Pawn)) AxisValue false))

(event Input|AxisEvents|InputAxisVistaX
  (params (AxisValue :type Float%20%28single-precision%29))
  (Pawn|Input|AddControllerYawInput AxisValue))

(event Input|AxisEvents|InputAxisVistaY
  (params (AxisValue :type Float%20%28single-precision%29))
  (Pawn|Input|AddControllerPitchInput AxisValue))

(fn ConstructionScript)